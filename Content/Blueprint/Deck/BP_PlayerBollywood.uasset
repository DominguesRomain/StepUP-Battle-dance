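; Bollywood-style player for a dance card game, holding that player's piles, hand reference and card-play count.
; On BeginPlay it gets its ID and manager from GM, places discard, deck and choreography-zone transforms for one of four seats, and copies the Bollywood deck.
; Helpers split cards by type into Pas and Figure decks, refill the Figure zone, and flag the UI at three cards played.
; Classic discard and passive functions are empty stubs.
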(event `self.ReceiveBeginPlay`
  (bind (_style _player _id) (`/Game/Blueprint/GM_StepUP.DefineActualPlayerManagerIDAndStyle` (`self.GM`)))
  (bind _output_get (set `self.IDjoueur/style` _id))
  (set `self.MyManager` _player)
  (`self.Emplacement DeckPas/Figure/Défausse` _output_get)
  (set `self.DeckBollywood` (`/Game/Blueprint/GM_StepUP.DeckBollywood` (`self.GM`))))

(fn `défausseClasique`)

(fn `Emplacement DeckPas/Figure/Défausse`
  (params (Selection :type Integer))
  (switch `int` Selection
    (:`1`
      (set `self.Défausse Transform` (`KismetMathLibrary.MakeTransform` (520.0 430.0 0.0) (struct :`Yaw` 90.0)))
      (set `self.DeckPasTransform` (`KismetMathLibrary.MakeTransform` (230.0 430.0 0.0) (struct :`Yaw` 90.0)))
      (set `self.DeckFigure Transform` (`KismetMathLibrary.MakeTransform` (-190.0 430.0 0.0) (struct :`Yaw` 90.0)))
      (set `self.MyZoneChoréTransform` (`KismetMathLibrary.MakeTransform` (0.0 180.0 0.0) (struct :`Yaw` 90.0))))
    (:`2`
      (set `self.Défausse Transform` (`KismetMathLibrary.MakeTransform` (430.0 -550.0 0.0)))
      (set `self.DeckPasTransform` (`KismetMathLibrary.MakeTransform` (430.0 -250.0 0.0)))
      (set `self.DeckFigure Transform` (`KismetMathLibrary.MakeTransform` (430.0 150.0 0.0)))
      (set `self.MyZoneChoréTransform` (`KismetMathLibrary.MakeTransform` (180.0 0.0 0.0))))
    (:`3`
      (set `self.Défausse Transform` (`KismetMathLibrary.MakeTransform` (-530.0 -430.0 0.0) (struct :`Yaw` -90.0)))
      (set `self.DeckPasTransform` (`KismetMathLibrary.MakeTransform` (-250.0 -430.0 0.0) (struct :`Yaw` -90.0)))
      (set `self.DeckFigure Transform` (`KismetMathLibrary.MakeTransform` (170.0 -430.0 0.0) (struct :`Yaw` -90.0)))
      (set `self.MyZoneChoréTransform` (`KismetMathLibrary.MakeTransform` (0.0 -180.0 0.0) (struct :`Yaw` -90.0))))
    (:`4`
      (set `self.Défausse Transform` (`KismetMathLibrary.MakeTransform` (-430.0 510.0 0.0) (struct :`Yaw` 180.0)))
      (set `self.DeckPasTransform` (`KismetMathLibrary.MakeTransform` (-429.0 220.0 0.0) (struct :`Yaw` 180.0)))
      (set `self.DeckFigure Transform` (`KismetMathLibrary.MakeTransform` (-430.0 -160.0 0.0) (struct :`Yaw` 180.0)))
      (set `self.MyZoneChoréTransform` (`KismetMathLibrary.MakeTransform` (0.0 180.0 0.0) (struct :`Yaw` 180.0))))))

(fn `GenrateZoneFigureCard`
  (locals (TailleZone :type Integer :default 2))
  (bind _deckfigure (`self.DeckFigure`))
  (bind _output (`|GetArrayItem` _deckfigure))
  (while (< (`KismetArrayLibrary.Array_Length` (`self.ZoneFigureCard`)) (`local.TailleZone`))
    (`KismetArrayLibrary.Array_Add` (`self.ZoneFigureCard`) _output)
    (`KismetArrayLibrary.Array_RemoveItem` _deckfigure _output)))

(fn `Gestion Carte Data Défausse`
  (params (cardInstance :type "/Game/Blueprint/ListeEtEnum/FCardInstanceDataBollywood Structure"))
  (`KismetArrayLibrary.Array_Add` (`self.PileDéfausse`) cardInstance))

(fn `GestionLimiteCarteJouéParTour`
  (bind _result (`/Engine/EditorBlueprintResources/StandardMacros.IncrementInt` (`self.CarteJoué`))
    (:`  `
      (if (>= _result 3)
        (set `/Game/Blueprint/Widget/WBPStyle/WBP_BollywoodHand.MaxCard` true (`/Game/Blueprint/GM_StepUP.WBP Bollywood` (`self.GM`)))))))

(fn `MyZoneChoréCardInst`
  (params (`cardInstChoré` :type "/Game/Blueprint/ListeEtEnum/FCardInstanceDataBollywood Structure"))
  (`KismetArrayLibrary.Array_Add` (`self.PileZoneChoré`) `cardInstChoré`))

(fn `PassifClassique`)

(fn `RefMain`
  (params (Main :type "Array of /Game/Blueprint/ListeEtEnum/FCardInstanceDataBollywood Structure"))
  (set `self.HandCarte` Main))

(fn `SplitDeckPas/Figure`
  (params (CardInstance :type "Array of /Game/Blueprint/ListeEtEnum/FCardInstanceDataBollywood Structure"))
  (bind (_sdatacard_cartetemplate _sdatacard_uniqueidguid _sdatacard_ownerid _sdatacard_hasbeenplayed _sdatacard_decknumber _sdatacard_deckstyle _sdatacard_location _sdatacard_isrecto_) (break `/Game/Blueprint/ListeEtEnum/FCardInstanceDataBollywood` (`self.SDataCard`)))
  (for _array_element CardInstance
    (bind _output_get (set `self.SDataCard` _array_element))
    (if (`|EnumEquality` (`self.EType`) (`/Game/Blueprint/ListeEtEnum/DA_CartesBollywood.CardType` (break `/Game/Blueprint/ListeEtEnum/FCardInstanceDataBollywood` _output_get)))
      (bind _output_get_2 (set `self.SDataCard` (make `/Game/Blueprint/ListeEtEnum/FCardInstanceDataBollywood` _sdatacard_cartetemplate _sdatacard_uniqueidguid _sdatacard_ownerid _sdatacard_hasbeenplayed _sdatacard_decknumber _sdatacard_deckstyle "NewEnumerator5" _sdatacard_isrecto_)))
      (`KismetArrayLibrary.Array_Add` (`self.DeckPas`) _output_get_2)
      (else
        (bind _output_get_3 (set `self.SDataCard` (make `/Game/Blueprint/ListeEtEnum/FCardInstanceDataBollywood` _sdatacard_cartetemplate _sdatacard_uniqueidguid _sdatacard_ownerid _sdatacard_hasbeenplayed _sdatacard_decknumber _sdatacard_deckstyle "NewEnumerator0" _sdatacard_isrecto_)))
        (`KismetArrayLibrary.Array_Add` (`self.DeckFigure`) _output_get_3)))))

(fn `UserConstructionScript`)