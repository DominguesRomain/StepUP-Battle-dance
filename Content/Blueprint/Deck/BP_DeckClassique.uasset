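; BP_DeckClassique is the "Classique" card deck, turning its DeckList into per-card instance data at BeginPlay.
; BuildDeckInstances gives each card a GUID, owner, deck number and style so it can carry its own data, reshuffling after every addition.
; SelectFirstDeckCard recursively advances a persistent index to a card whose Location is the first enum value, returning its index.
; HandREf stores a reference to the hand.
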(event `self.ReceiveBeginPlay`
  (`self.BuildDeckInstances` (`self.DeckList`)))

(fn `BuildDeckInstances`
  (params (decklist :type "Array of /Game/Blueprint/ListeEtEnum/DA_CartesClassique Object Reference"))
  (returns (CardInstanceData :type "Array of /Game/Blueprint/ListeEtEnum/FCardInstanceDataClassique Structure"))
  (bind _returnvalue (`KismetGuidLibrary.NewGuid`))
  ; Créer le deck: enregistre chaque carte dans un deck instance avec un GUID pour que les cartes puisse porté leur donné (vois a évolué en fonction des efets lié au cartes)
  (for (_array_element _array_index) decklist
    (if (`KismetGuidLibrary.IsValid_Guid` _returnvalue) :!label _label
      (`KismetArrayLibrary.Array_Add` (`self.DeckCardInstanceData`) (make `/Game/Blueprint/ListeEtEnum/FCardInstanceDataClassique` _array_element (`KismetGuidLibrary.Conv_GuidToString` _returnvalue) (`/Game/Blueprint/GM_StepUP.PlayerID` (`self.GM`)) false _array_index "Clasique"))
      (`self.DeckShuffle`)
      (else
        (`KismetSystemLibrary.PrintString` "Invalidate GUID" true true (struct :`R` 0.557292 :`B` 0.024246 :`A` 1.0))
        (`KismetGuidLibrary.Invalidate_Guid` _returnvalue)
        (goto _label))))
  (return (`self.DeckCardInstanceData`)))

(fn `DeckShuffle`
  (`KismetArrayLibrary.Array_Shuffle` (`self.DeckCardInstanceData`)))

(fn `HandREf`
  (params (NewParam :type "/Game/Blueprint/Widget/WBPStyle/WBP_ClassiqueHand Object Reference"))
  (set `self.HandClassique` NewParam))

(fn `SelectFirstDeckCard`
  (returns (Find :type Integer))
  (bind _output (`|GetArrayItem` (`self.DeckCardInstanceData`) (`self.FirtDeckCardInt`)))
  ; Choisi Une carte présente dans le deck
  (bind _output_get (set `self.SelectedCard` _output))
  (if (`|EnumEquality` "NewEnumerator0" (`.Location_24_21FD5B7F4DF98A505664BC8E65D884DB` (break `/Game/Blueprint/ListeEtEnum/FCardInstanceDataClassique` _output_get)))
    (return (`KismetArrayLibrary.Array_Find` (`self.DeckCardInstanceData`) _output))
    (else
      (`/Engine/EditorBlueprintResources/StandardMacros.IncrementInt` (`self.FirtDeckCardInt`)
        (:`  `
          (`self.SelectFirstDeckCard`))))))

(fn `UserConstructionScript`)