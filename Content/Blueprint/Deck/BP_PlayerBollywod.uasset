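; BP_PlayerBollywod is the Bollywood-style player in a card game, holding that player's step (Pas), figure and discard pile setup.
; On BeginPlay it gets its ID and manager from GM, picks hard-coded pile transforms for one of four table sides, and copies GM's Bollywood deck.
; SplitDeckPasFigure, not called here, sorts card instances by type into Pas and Figure decks, rewriting each card's last enum field.
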(event `self.ReceiveBeginPlay`
  (bind (_style _player _id) (`/Game/Blueprint/GM_StepUP.DefineActualPlayerManagerIDAndStyle` (`self.GM`)))
  (bind _output_get (set `self.IDjoueur/style` _id))
  (set `self.MyManager` _player)
  (`self.Emplacement DeckPas/Figure/Défausse` _output_get)
  (set `self.DEckBolly` (`/Game/Blueprint/GM_StepUP.DeckBollywood` (`self.GM`))))

(fn `Emplacement DeckPas/Figure/Défausse`
  (params (Selection :type Integer))
  (switch `int` Selection
    (:`1`
      (set `self.Défausse Transform` (`KismetMathLibrary.MakeTransform` (520.0 430.0 0.0) (struct :`Yaw` 90.0)))
      (set `self.DeckPasTransform` (`KismetMathLibrary.MakeTransform` (230.0 430.0 0.0) (struct :`Yaw` 90.0)))
      (set `self.DeckFigure Transform` (`KismetMathLibrary.MakeTransform` (-190.0 430.0 0.0) (struct :`Yaw` 90.0))))
    (:`2`
      (set `self.Défausse Transform` (`KismetMathLibrary.MakeTransform` (430.0 -550.0 0.0)))
      (set `self.DeckPasTransform` (`KismetMathLibrary.MakeTransform` (430.0 -250.0 0.0)))
      (set `self.DeckFigure Transform` (`KismetMathLibrary.MakeTransform` (430.0 150.0 0.0))))
    (:`3`
      (set `self.Défausse Transform` (`KismetMathLibrary.MakeTransform` (-530.0 -430.0 0.0) (struct :`Yaw` -90.0)))
      (set `self.DeckPasTransform` (`KismetMathLibrary.MakeTransform` (-250.0 -430.0 0.0) (struct :`Yaw` -90.0)))
      (set `self.DeckFigure Transform` (`KismetMathLibrary.MakeTransform` (170.0 -430.0 0.0) (struct :`Yaw` -90.0))))
    (:`4`
      (set `self.Défausse Transform` (`KismetMathLibrary.MakeTransform` (-430.0 510.0 0.0) (struct :`Yaw` 180.0)))
      (set `self.DeckPasTransform` (`KismetMathLibrary.MakeTransform` (-429.0 220.0 0.0) (struct :`Yaw` 180.0)))
      (set `self.DeckFigure Transform` (`KismetMathLibrary.MakeTransform` (-430.0 -160.0 0.0) (struct :`Yaw` 180.0))))))

(fn `SplitDeckPas/Figure`
  (params (CardInstance :type "Array of /Game/Blueprint/ListeEtEnum/FCardInstanceDataBollywood Structure"))
  (bind (_sdatacard_cartetemplate _sdatacard_uniqueid _sdatacard_ownerid _sdatacard_hasbeenplayed _sdatacard_decknumber _sdatacard_decksyle) (break `/Game/Blueprint/ListeEtEnum/FCardInstanceDataBollywood` (`self.SDataCard`)))
  (for _array_element CardInstance
    (bind _output_get (set `self.SDataCard` _array_element))
    (if (`|EnumEquality` (`self.EType`) (`/Game/Blueprint/ListeEtEnum/DA_CartesBollywood.CardType` (break `/Game/Blueprint/ListeEtEnum/FCardInstanceDataBollywood` _output_get)))
      (bind _output_get_2 (set `self.SDataCard` (make `/Game/Blueprint/ListeEtEnum/FCardInstanceDataBollywood` _sdatacard_cartetemplate _sdatacard_uniqueid _sdatacard_ownerid _sdatacard_hasbeenplayed _sdatacard_decknumber _sdatacard_decksyle "NewEnumerator5")))
      (`KismetArrayLibrary.Array_Add` (`self.DeckPas`) _output_get_2)
      (else
        (bind _output_get_3 (set `self.SDataCard` (make `/Game/Blueprint/ListeEtEnum/FCardInstanceDataBollywood` _sdatacard_cartetemplate _sdatacard_uniqueid _sdatacard_ownerid _sdatacard_hasbeenplayed _sdatacard_decknumber _sdatacard_decksyle)))
        (`KismetArrayLibrary.Array_Add` (`self.DeckFigure`) _output_get_3))))
  (`KismetSystemLibrary.PrintString` "Split End"))

(fn `UserConstructionScript`)