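; Bollywood-style deck for a card game, which builds the player's card instances at BeginPlay.
; Each DeckList template becomes an instance struct with a GUID, owner ID, deck number and location, so cards can carry their own data.
; The array reshuffles after every add, then PlayerBollywood splits it into Pas and Figure decks.
; Selection functions pick the card at a stored index in either of the player's decks.
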(event `self.ReceiveBeginPlay`
  (bind _cardinstancedata (`self.BuildDeckInstances` (`self.DeckList`)))
  (bind _output_get (set `self.Player Bollywood` (`/Game/Blueprint/GM_StepUP.PlayerBollywood` (`self.GM`))))
  (`/Game/Blueprint/DeckAndPlayer/BP_PlayerBollywood.SplitDeckPas/Figure` _output_get _cardinstancedata))

(fn `BuildDeckInstances`
  (params (decklist :type "Array of /Game/Blueprint/ListeEtEnum/DA_Cartes Object Reference"))
  (returns (CardInstanceData :type "Array of /Game/Blueprint/ListeEtEnum/FCardInstanceDataBollywood Structure"))
  (bind _returnvalue (`KismetGuidLibrary.NewGuid`))
  ; Créer le deck: enregistre chaque carte dans un deck instance avec un GUID pour que les cartes puisse porté leur donné (vois a évolué en fonction des efets lié au cartes)
  (for (_array_element _array_index) decklist
    (if (`KismetGuidLibrary.IsValid_Guid` _returnvalue) :!label _label
      (`KismetArrayLibrary.Array_Add` (`self.DeckCardInstanceData`) (make `/Game/Blueprint/ListeEtEnum/FCardInstanceDataBollywood` _array_element (`KismetGuidLibrary.Conv_GuidToString` _returnvalue) (`/Game/Blueprint/GM_StepUP.PlayerID` (`self.GM`)) false _array_index "Bollywood" "NewEnumerator5"))
      (`self.DeckShuffle`)
      (else
        (`KismetSystemLibrary.PrintString` "Invalidate GUID" true true (struct :`R` 0.557292 :`B` 0.024246 :`A` 1.0))
        (`KismetGuidLibrary.Invalidate_Guid` _returnvalue)
        (goto _label))))
  (return (`self.DeckCardInstanceData`)))

(fn `DeckShuffle`
  (`KismetArrayLibrary.Array_Shuffle` (`self.DeckCardInstanceData`)))

(fn `SelectFirstDeckCardFigure`
  (returns (Find :type Integer))
  (bind _deckfigure (`/Game/Blueprint/DeckAndPlayer/BP_PlayerBollywood.DeckFigure` (`self.Player Bollywood`)))
  (bind _output (`|GetArrayItem` _deckfigure (`self.FirtDeckCardInt`)))
  ; Choisi Une carte présente dans le deck
  (set `self.SelectedCard` _output)
  (return (`KismetArrayLibrary.Array_Find` _deckfigure _output)))

(fn `SelectFirstDeckCardPas`
  (returns (Find :type Integer))
  (bind _deckpas (`/Game/Blueprint/DeckAndPlayer/BP_PlayerBollywood.DeckPas` (`self.Player Bollywood`)))
  (bind _output (`|GetArrayItem` _deckpas (`self.FirtDeckCardInt`)))
  ; Choisi Une carte présente dans le deck
  (set `self.SelectedCard` _output)
  (return (`KismetArrayLibrary.Array_Find` _deckpas _output)))

(fn `UserConstructionScript`)