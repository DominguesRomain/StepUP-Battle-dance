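; BP_DeckClassique builds the Classique player's card deck at BeginPlay from DeckList.
; It spawns a BP_Cartes actor per entry at the Pas deck transform, pairing it with instance data and the template's effect component.
; The shuffled instance array goes to PlayerClassique's SplitDeckPasFigure, which receives it for the Pas/Figure split.
; Helper functions select a card at a stored index from the player's Pas or Figure deck.
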(event `self.ReceiveBeginPlay`
  (bind _cardinstancedata (`self.BuildDeckInstances` (`self.DeckList`)))
  (bind _output_get (set `self.Player Classique` (`/Game/Blueprint/GM_StepUP.PlayerClassique` (`self.GM`))))
  (`/Game/Blueprint/DeckAndPlayer/BP_PlayerClassique.SplitDeckPas/Figure` _output_get _cardinstancedata))

(fn `BuildDeckInstances`
  (params (decklist :type "Array of /Game/Blueprint/ListeEtEnum/DA_Cartes Object Reference"))
  (returns (CardInstanceData :type "Array of /Game/Blueprint/ListeEtEnum/FCardInstanceData Structure"))
  (locals (`FCard Instance Data` :type "/Game/Blueprint/ListeEtEnum/FCardInstanceData Structure"))
  (bind (_fcard_instance_data_cartetemplate _fcard_instance_data_ownerid _fcard_instance_data_decknumber _fcard_instance_data_deckstyle _fcard_instance_data_location _fcard_instance_data_isrecto_) (break `/Game/Blueprint/ListeEtEnum/FCardInstanceData` (`local.FCard Instance Data`)))
  (bind _fcard_instance_data_cartetemplate_2 (break `/Game/Blueprint/ListeEtEnum/FCardInstanceData` (`local.FCard Instance Data`)))
  ; Créer le deck: enregistre chaque carte dans un deck instance avec un GUID pour que les cartes puisse porté leur donné (vois a évolué en fonction des efets lié au cartes)
  (for (_array_element _array_index) decklist
    (set `local.FCard Instance Data` (make `/Game/Blueprint/ListeEtEnum/FCardInstanceData` _array_element (`/Game/Blueprint/GM_StepUP.PlayerID` (`self.GM`)) _array_index "NewEnumerator3" "NewEnumerator5" true null))
    (bind _returnvalue (`|SpawnActorFromClass` "/Game/Blueprint/BP_Cartes.BP_Cartes_C" (`/Game/Blueprint/DeckAndPlayer/BP_PlayerClassique.DeckPasTransform` (`self.Player Classique`)) "AlwaysSpawn" "MultiplyWithRoot" null "NewEnumerator3" (`/Game/Blueprint/ListeEtEnum/DA_Cartes.ComponentCardEffect` _fcard_instance_data_cartetemplate_2) (`self.GM`) false (`local.FCard Instance Data`) null))
    (bind _output_get (set `local.FCard Instance Data` (make `/Game/Blueprint/ListeEtEnum/FCardInstanceData` _fcard_instance_data_cartetemplate _fcard_instance_data_ownerid _fcard_instance_data_decknumber _fcard_instance_data_deckstyle _fcard_instance_data_location _fcard_instance_data_isrecto_ _returnvalue)))
    (`KismetArrayLibrary.Array_Add` (`self.DeckCardInstanceData`) _output_get)
    (`self.DeckShuffle`))
  (`self.DeckShuffle`)
  (return (`self.DeckCardInstanceData`)))

(fn `DeckShuffle`
  (`KismetArrayLibrary.Array_Shuffle` (`self.DeckCardInstanceData`)))

(fn `SelectFirstDeckCardFigure`
  (returns (Find :type Integer))
  (bind _deckfigure (`/Game/Blueprint/DeckAndPlayer/BP_PlayerClassique.DeckFigure` (`self.Player Classique`)))
  (bind _output (`|GetArrayItem` _deckfigure (`self.FirtDeckCardInt`)))
  ; Choisi Une carte présente dans le deck
  (set `self.SelectedCard` _output)
  (return (`KismetArrayLibrary.Array_Find` _deckfigure _output)))

(fn `SelectFirstDeckCardPas`
  (returns (Find :type Integer))
  (bind _deckpas (`/Game/Blueprint/DeckAndPlayer/BP_PlayerClassique.DeckPas` (`self.Player Classique`)))
  (bind _output (`|GetArrayItem` _deckpas (`self.FirtDeckCardInt`)))
  ; Choisi Une carte présente dans le deck
  (set `self.SelectedCard` _output)
  (return (`KismetArrayLibrary.Array_Find` _deckpas _output)))

(fn `UserConstructionScript`)