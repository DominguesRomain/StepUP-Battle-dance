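; Bollywood-style player in a card game, owning the Pas and Figure decks, Figure zone, discard and choreography piles.
; BeginPlay places its zones by player ID, and cards split by type into the two decks.
; Played cards move to the shared Piste and choreography pile, with a per-turn limit flag.
; Its passive accumulates Adeptes; reaching ten triggers a draw, Pas shuffle, automatic Figure and Pas plays, and a zone refill.
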(event `self.ReceiveBeginPlay`
  (bind (_style _player _id) (`/Game/Blueprint/GM_StepUP.DefineActualPlayerManagerIDAndStyle` (`self.GM`)))
  (bind _output_get (set `self.IDjoueur/style` _id))
  (set `self.MyManager` _player)
  (`self.Emplacement DeckPas/Figure/Défausse` _output_get)
  (set `self.DeckBollywood` (`/Game/Blueprint/GM_StepUP.DeckBollywood` (`self.GM`))))

(fn `Emplacement DeckPas/Figure/Défausse`
  (params (Selection :type Integer))
  (switch `int` Selection
    (:`1`
      (set `self.Défausse Transform` (`KismetMathLibrary.MakeTransform` (520.0 430.0 0.0) (struct :`Yaw` 90.0)))
      (set `self.DeckPasTransform` (`KismetMathLibrary.MakeTransform` (230.0 430.0 0.0) (struct :`Yaw` 90.0)))
      (set `self.DeckFigure Transform` (`KismetMathLibrary.MakeTransform` (-190.0 430.0 0.0) (struct :`Yaw` 90.0)))
      (set `self.MyZoneChoréTransform` (`KismetMathLibrary.MakeTransform` (0.0 180.0 0.0) (struct :`Yaw` 90.0)))
      (set `self.handTransform` (`KismetMathLibrary.MakeTransform` (-20.0 430.0 0.0) (struct :`Yaw` 90.0))))
    (:`2`
      (set `self.Défausse Transform` (`KismetMathLibrary.MakeTransform` (430.0 -550.0 0.0)))
      (set `self.DeckPasTransform` (`KismetMathLibrary.MakeTransform` (430.0 -250.0 0.0)))
      (set `self.DeckFigure Transform` (`KismetMathLibrary.MakeTransform` (430.0 150.0 0.0)))
      (set `self.MyZoneChoréTransform` (`KismetMathLibrary.MakeTransform` (180.0 0.0 0.0)))
      (set `self.handTransform` (`KismetMathLibrary.MakeTransform` (430.0 0.0 0.0))))
    (:`3`
      (set `self.Défausse Transform` (`KismetMathLibrary.MakeTransform` (-530.0 -430.0 0.0) (struct :`Yaw` -90.0)))
      (set `self.DeckPasTransform` (`KismetMathLibrary.MakeTransform` (-250.0 -430.0 0.0) (struct :`Yaw` -90.0)))
      (set `self.DeckFigure Transform` (`KismetMathLibrary.MakeTransform` (170.0 -430.0 0.0) (struct :`Yaw` -90.0)))
      (set `self.MyZoneChoréTransform` (`KismetMathLibrary.MakeTransform` (0.0 -180.0 0.0) (struct :`Yaw` -90.0)))
      (set `self.handTransform` (`KismetMathLibrary.MakeTransform` (20.0 -430.0 0.0) (struct :`Yaw` -90.0))))
    (:`4`
      (set `self.Défausse Transform` (`KismetMathLibrary.MakeTransform` (-430.0 510.0 0.0) (struct :`Yaw` 180.0)))
      (set `self.DeckPasTransform` (`KismetMathLibrary.MakeTransform` (-429.0 220.0 0.0) (struct :`Yaw` 180.0)))
      (set `self.DeckFigure Transform` (`KismetMathLibrary.MakeTransform` (-430.0 -160.0 0.0) (struct :`Yaw` 180.0)))
      (set `self.MyZoneChoréTransform` (`KismetMathLibrary.MakeTransform` (0.0 180.0 0.0) (struct :`Yaw` 180.0)))
      (set `self.handTransform` (`KismetMathLibrary.MakeTransform` (-430.0 -10.0 0.0) (struct :`Yaw` 180.0))))))

(fn `FigureCardPlayFromDeck`
  (params (find :type Integer))
  (locals (`Card Instance Bollywood` :type "/Game/Blueprint/ListeEtEnum/FCardInstanceData Structure") (NewLocalVar :type "Transform Structure"))
  (bind _card_instance_bollywood (`local.Card Instance Bollywood`))
  (bind (_cardboxtransfom_location _cardboxtransfom_rotation _cardboxtransfom_scale) (`KismetMathLibrary.BreakTransform` (`/Game/Blueprint/BP_PisteEtChoré.CardBoxTransfom` (`/Game/Blueprint/GM_StepUP.BP_Piste` (`self.GM`)))))
  (bind _output_get (set `local.Card Instance Bollywood` (`|GetArrayItem` (`self.DeckFigure`) find)))
  (bind _output_get_2 (set `local.Card Instance Bollywood` (make `/Game/Blueprint/ListeEtEnum/FCardInstanceData` (break `/Game/Blueprint/ListeEtEnum/FCardInstanceData` _output_get) (`.OwnerID_10_6FF36D9A48E4EF047131B28C579EED57` (break `/Game/Blueprint/ListeEtEnum/FCardInstanceData` _output_get)) (`.DeckNumber_17_0DE01F88464E1E8634D709B000A51AF6` (break `/Game/Blueprint/ListeEtEnum/FCardInstanceData` _output_get)) (`.DeckStyle_32_FDB562A746448077DCE221999F391151` (break `/Game/Blueprint/ListeEtEnum/FCardInstanceData` _output_get)) "NewEnumerator2" true (`.BP_Carte_31_A73927C24E172773FC43A29CF6C4A8E9` (break `/Game/Blueprint/ListeEtEnum/FCardInstanceData` _output_get)))))
  (`/Game/Blueprint/BP_PisteEtChoré.GestionAddToPLayerPiste` (`/Game/Blueprint/GM_StepUP.BP_Piste` (`self.GM`)) (`.DeckStyle_32_FDB562A746448077DCE221999F391151` (break `/Game/Blueprint/ListeEtEnum/FCardInstanceData` _output_get)) _output_get_2)
  (`/Game/Blueprint/BP_Cartes.CardNewPlace` (`.BP_Carte_31_A73927C24E172773FC43A29CF6C4A8E9` (break `/Game/Blueprint/ListeEtEnum/FCardInstanceData` _output_get)) (`KismetMathLibrary.MakeTransform` _cardboxtransfom_location _cardboxtransfom_rotation (* _cardboxtransfom_scale (7.0 8.0 6.0))) _output_get_2)
  (`self.MyZoneChoréCardInst` (`/Game/Blueprint/GM_StepUP.PlayerBollywood` (`self.GM`)) _card_instance_bollywood)
  (`KismetArrayLibrary.Array_RemoveItem` (`self.DeckFigure`) _card_instance_bollywood))

(fn `FigureCardPlayFromZone`
  (params (find :type Integer))
  (locals (`Card Instance Bollywood` :type "/Game/Blueprint/ListeEtEnum/FCardInstanceData Structure"))
  (bind _card_instance_bollywood (`local.Card Instance Bollywood`))
  (bind (_cardboxtransfom_location _cardboxtransfom_rotation _cardboxtransfom_scale) (`KismetMathLibrary.BreakTransform` (`/Game/Blueprint/BP_PisteEtChoré.CardBoxTransfom` (`/Game/Blueprint/GM_StepUP.BP_Piste` (`self.GM`)))))
  (bind _output_get (set `local.Card Instance Bollywood` (`|GetArrayItem` (`self.ZoneFigureCard`) find)))
  (bind _output_get_2 (set `local.Card Instance Bollywood` (make `/Game/Blueprint/ListeEtEnum/FCardInstanceData` (break `/Game/Blueprint/ListeEtEnum/FCardInstanceData` _output_get) (`.OwnerID_10_6FF36D9A48E4EF047131B28C579EED57` (break `/Game/Blueprint/ListeEtEnum/FCardInstanceData` _output_get)) (`.DeckNumber_17_0DE01F88464E1E8634D709B000A51AF6` (break `/Game/Blueprint/ListeEtEnum/FCardInstanceData` _output_get)) (`.DeckStyle_32_FDB562A746448077DCE221999F391151` (break `/Game/Blueprint/ListeEtEnum/FCardInstanceData` _output_get)) "NewEnumerator2" (`.IsRecto?_28_63F5495E469FDE489E753FAFE753AA19` (break `/Game/Blueprint/ListeEtEnum/FCardInstanceData` _output_get)) (`.BP_Carte_31_A73927C24E172773FC43A29CF6C4A8E9` (break `/Game/Blueprint/ListeEtEnum/FCardInstanceData` _output_get)))))
  (`/Game/Blueprint/BP_PisteEtChoré.GestionAddToPLayerPiste` (`/Game/Blueprint/GM_StepUP.BP_Piste` (`self.GM`)) (`.DeckStyle_32_FDB562A746448077DCE221999F391151` (break `/Game/Blueprint/ListeEtEnum/FCardInstanceData` _output_get)) _output_get_2)
  (`/Game/Blueprint/BP_Cartes.CardNewPlace` (`.BP_Carte_31_A73927C24E172773FC43A29CF6C4A8E9` (break `/Game/Blueprint/ListeEtEnum/FCardInstanceData` _output_get)) (`KismetMathLibrary.MakeTransform` _cardboxtransfom_location _cardboxtransfom_rotation (* _cardboxtransfom_scale (7.0 8.0 6.0))) _output_get_2)
  (`self.MyZoneChoréCardInst` (`/Game/Blueprint/GM_StepUP.PlayerBollywood` (`self.GM`)) _card_instance_bollywood)
  (`KismetArrayLibrary.Array_RemoveItem` (`self.ZoneFigureCard`) _card_instance_bollywood))

(fn `FromRandomBoardVersoToDéfausse`
  (params (carteVersoB :type "Array of /Game/Blueprint/ListeEtEnum/FCardInstanceData Structure"))
  (locals (`Card Instance ` :type "/Game/Blueprint/ListeEtEnum/FCardInstanceData Structure"))
  (bind _returnvalue (`KismetArrayLibrary.Array_Length` carteVersoB))
  (if (> _returnvalue 0)
    (bind _output_get (set `local.Card Instance ` (`|GetArrayItem` carteVersoB (`KismetMathLibrary.RandomInteger` (- _returnvalue 1)))))
    (message `/Game/Blueprint/BPI/BPI_WidgetInter.CardDestroy` (`.BP_Carte_31_A73927C24E172773FC43A29CF6C4A8E9` (break `/Game/Blueprint/ListeEtEnum/FCardInstanceData` _output_get)) (`.BP_Carte_31_A73927C24E172773FC43A29CF6C4A8E9` (break `/Game/Blueprint/ListeEtEnum/FCardInstanceData` _output_get)))
    (return)))

(fn `GenrateZoneFigureCard`
  (locals (TailleZone :type Integer :default 2))
  (bind _deckfigure (`self.DeckFigure`))
  (bind _output (`|GetArrayItem` _deckfigure))
  (while (< (`KismetArrayLibrary.Array_Length` (`self.ZoneFigureCard`)) (`local.TailleZone`))
    (`KismetArrayLibrary.Array_Add` (`self.ZoneFigureCard`) _output)
    (`KismetArrayLibrary.Array_RemoveItem` _deckfigure _output)))

(fn `Gestion Carte Data Défausse`
  (params (cardInstance :type "/Game/Blueprint/ListeEtEnum/FCardInstanceData Structure"))
  (`KismetArrayLibrary.Array_Add` (`self.PileDéfausse`) cardInstance))

(fn `GestionLimiteCarteJouéParTour`
  (bind _result (`/Engine/EditorBlueprintResources/StandardMacros.IncrementInt` (`self.CarteJoué`))
    (:`  `
      (if (>= _result 3)
        (set `/Game/Blueprint/Widget/WBPStyle/WBP_BollywoodHand.MaxCard` true (`/Game/Blueprint/GM_StepUP.WBP Bollywood` (`self.GM`)))))))

(fn `MyZoneChoréCardInst`
  (params (`cardInstChoré` :type "/Game/Blueprint/ListeEtEnum/FCardInstanceData Structure"))
  (`KismetArrayLibrary.Array_Add` (`self.PileZoneChoré`) `cardInstChoré`))

(fn `PasCardPlayFromDeck`
  (params (find :type Integer))
  (locals (`Card Instance Bollywood` :type "/Game/Blueprint/ListeEtEnum/FCardInstanceData Structure"))
  (bind _card_instance_bollywood (`local.Card Instance Bollywood`))
  (bind (_output_cartetemplate _output_ownerid _output_decknumber _output_deckstyle _output_location _output_isrecto_ _output_bp_carte) (break `/Game/Blueprint/ListeEtEnum/FCardInstanceData` (`|GetArrayItem` (`self.DeckPas`) find)))
  (bind (_cardboxtransfom_location _cardboxtransfom_rotation _cardboxtransfom_scale) (`KismetMathLibrary.BreakTransform` (`/Game/Blueprint/BP_PisteEtChoré.CardBoxTransfom` (`/Game/Blueprint/GM_StepUP.BP_Piste` (`self.GM`)))))
  (bind _output_get (set `local.Card Instance Bollywood` (make `/Game/Blueprint/ListeEtEnum/FCardInstanceData` _output_cartetemplate _output_ownerid _output_decknumber _output_deckstyle "NewEnumerator2" false _output_bp_carte)))
  (`/Game/Blueprint/BP_PisteEtChoré.GestionAddToPLayerPiste` (`/Game/Blueprint/GM_StepUP.BP_Piste` (`self.GM`)) _output_deckstyle _output_get)
  (`/Game/Blueprint/BP_Cartes.CardNewPlace` _output_bp_carte (`KismetMathLibrary.MakeTransform` _cardboxtransfom_location _cardboxtransfom_rotation (* _cardboxtransfom_scale (7.0 8.0 6.0))) _output_get)
  (`self.MyZoneChoréCardInst` (`/Game/Blueprint/GM_StepUP.PlayerBollywood` (`self.GM`)) _card_instance_bollywood)
  (`KismetArrayLibrary.Array_RemoveItem` (`self.DeckPas`) _card_instance_bollywood))

(fn `PassifAdeptesCount`
  (params (ValueAdpetesTransform :type Integer))
  (bind _adeptesbollywood (`self.AdeptesBollywood`))
  (set `self.OldAdeptesValue` _adeptesbollywood)
  (set `self.AdeptesBollywood` (+ _adeptesbollywood ValueAdpetesTransform))
  (`self.PassifBollywoodInGame`))

(fn `PassifBollywoodEndGame`)

(fn `PassifBollywoodInGame`
  (bind _gm (`self.GM`))
  (bind _deckbollywood (`/Game/Blueprint/GM_StepUP.DeckBollywood` _gm))
  ;[0 0.8353 0.8627 0.502] Passif Bollywood In Game
  (if (< (`self.OldAdeptesValue`) 10)
    (if (> (`self.AdeptesBollywood`) 9)
      (`/Game/Blueprint/Widget/WBPStyle/WBP_BollywoodHand.DrawAction` (`/Game/Blueprint/GM_StepUP.WBP Bollywood` _gm) 2)
      (`self.ShufflePas`)
      (bind _find (`/Game/Blueprint/DeckAndPlayer/BP_DeckBollywood.SelectFirstDeckCardFigure` _deckbollywood))
      (`self.FigureCardPlayFromDeck` _find)
      (bind _find_2 (`/Game/Blueprint/DeckAndPlayer/BP_DeckBollywood.SelectFirstDeckCardPas` _deckbollywood))
      (`self.PasCardPlayFromDeck` _find_2)
      (`self.GenrateZoneFigureCard`))))

(fn `PassifDéfausseBollywood`
  ;[0 0.8353 0.8627 0.502] Passif Bollywood
  (`self.PassifAdeptesCount` 4))

(fn `ReadAndActiveCardEffect`
  (params (Card :type "/Game/Blueprint/BP_Cartes Object Reference"))
  (bind _output_get (set `self.Card` Card))
  (`ActorComponent.Activate` (`self.FindComponentByTag` _output_get "/Game/Blueprint/BPC/ComponentCardEffect.ComponentCardEffect_C" "CardEffect") true))

(fn `RefMain`
  (params (Main :type "Array of /Game/Blueprint/ListeEtEnum/FCardInstanceData Structure"))
  (set `self.HandCarte` Main))

(fn `ShufflePas`
  (`KismetArrayLibrary.Array_Shuffle` (`self.DeckPas`)))

(fn `SplitDeckPas/Figure`
  (params (CardInstance :type "Array of /Game/Blueprint/ListeEtEnum/FCardInstanceData Structure"))
  (bind (_sdatacard_cartetemplate _sdatacard_ownerid _sdatacard_decknumber _sdatacard_deckstyle _sdatacard_location _sdatacard_isrecto_ _sdatacard_bp_carte) (break `/Game/Blueprint/ListeEtEnum/FCardInstanceData` (`self.SDataCard`)))
  (for _array_element CardInstance
    (bind _output_get (set `self.SDataCard` _array_element))
    (if (`|EnumEquality` (`self.EType`) (`/Game/Blueprint/ListeEtEnum/DA_Cartes.CardType` (break `/Game/Blueprint/ListeEtEnum/FCardInstanceData` _output_get)))
      (bind _output_get_2 (set `self.SDataCard` (make `/Game/Blueprint/ListeEtEnum/FCardInstanceData` _sdatacard_cartetemplate _sdatacard_ownerid _sdatacard_decknumber _sdatacard_deckstyle "NewEnumerator5" _sdatacard_isrecto_ _sdatacard_bp_carte)))
      (`KismetArrayLibrary.Array_Add` (`self.DeckPas`) _output_get_2)
      (else
        (bind _output_get_3 (set `self.SDataCard` (make `/Game/Blueprint/ListeEtEnum/FCardInstanceData` _sdatacard_cartetemplate _sdatacard_ownerid _sdatacard_decknumber _sdatacard_deckstyle "NewEnumerator0" _sdatacard_isrecto_ _sdatacard_bp_carte)))
        (`KismetArrayLibrary.Array_Add` (`self.DeckFigure`) _output_get_3)))))

(fn `UserConstructionScript`)