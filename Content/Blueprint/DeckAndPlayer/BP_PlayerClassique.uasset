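; BP_PlayerClassique is the Classique-style player in a dance-themed card game, holding its decks, hand, discard, choreography pile, Posture tokens and Adeptes score.
; BeginPlay takes the player ID from the GameMode to position card zones and fetch the deck, which splits into Pas and Figure piles.
; GestionnaireDeChoix routes choices to the Posture-paid passive or named card effects, including removing face-down cards from any player's board.
; Card effects run by activating tagged components.
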(event `self.ReceiveBeginPlay`
  (bind (_style _player _id) (`/Game/Blueprint/GM_StepUP.DefineActualPlayerManagerIDAndStyle` (`self.GM`)))
  (bind _output_get (set `self.IDjoueur/style` _id))
  (set `self.MyManager` _player)
  (`self.Emplacement DeckPas/Figure/Défausse` _output_get)
  (set `self.DeckClasique` (`/Game/Blueprint/GM_StepUP.DeckClassique` (`self.GM`))))

(fn `ActivateFigureEffect`
  (params (Cartedata :type "/Game/Blueprint/ListeEtEnum/FCardInstanceDataClassique Structure")))

(fn `DéfausseFonction`
  (params (carte :type "/Game/Blueprint/Widget/WBP_Cartes Object Reference"))
  (locals (`Card Instance Classique` :type "/Game/Blueprint/ListeEtEnum/FCardInstanceDataClassique Structure"))
  (bind (_cardinstanceclassique_cartetemplate _cardinstanceclassique_uniqueidguid _cardinstanceclassique_ownerid _cardinstanceclassique_hasbeenplayed _cardinstanceclassique_decknumber _cardinstanceclassique_deckstyle _cardinstanceclassique_location _cardinstanceclassique_isrecto_) (break `/Game/Blueprint/ListeEtEnum/FCardInstanceDataClassique` (`/Game/Blueprint/Widget/WBP_Cartes.CardInstanceClassique` carte)))
  (bind _output_get (set `local.Card Instance Classique` (make `/Game/Blueprint/ListeEtEnum/FCardInstanceDataClassique` _cardinstanceclassique_cartetemplate _cardinstanceclassique_uniqueidguid _cardinstanceclassique_ownerid _cardinstanceclassique_hasbeenplayed _cardinstanceclassique_decknumber _cardinstanceclassique_deckstyle "NewEnumerator3" _cardinstanceclassique_isrecto_)))
  (`Widget.RemoveFromParent` carte)
  (`|SpawnActorFromClass` "/Game/Blueprint/BP_Cartes.BP_Cartes_C" (`self.Défausse Transform`) "Undefined" "MultiplyWithRoot" null (struct) (struct) _output_get (struct) "NewEnumerator3" null (`self.GM`) false null))

(fn `défaussePassifClasique`
  (params (`Value Choix` :type Integer))
  (locals (Posture :type Integer))
  (bind _value (`BlueprintMapLibrary.Map_Find` (`self.Jeton`) "Posture"))
  ;[0.902 0.2196 0.6588 0.502] Passif de défausse classique
  (switch `int` `Value Choix`
    (:`1`
      (if (> _value 0)
        (`self.PostureAddValue` -1
          (:`  `
            (bind _find (`/Game/Blueprint/DeckAndPlayer/BP_DeckClassique.SelectFirstDeckCardFigure` (`/Game/Blueprint/GM_StepUP.DeckClassique` (`self.GM`))))
            (`self.FigureCardPlayFromDeck` _find)
            (`self.GenrateZoneFigureCard`)))
        (else
          (`KismetSystemLibrary.PrintString` "Pas Assez de jeton" :!label _label))))
    (:`2`
      (if (> _value 1)
        (`self.PostureAddValue` -2
          (:`  `
            (`/Game/Blueprint/Widget/WBPStyle/WBP_ClassiqueHand.DrawAction` (`/Game/Blueprint/GM_StepUP.WBP Classique` (`self.GM`)) 3)
            (`self.ShufflePas`)))
        (else
          (goto _label))))))

(fn `ElegantEffect`
  (params (ChoixValue :type Integer))
  (locals (Value :type Integer))
  (bind _value (`local.Value`))
  (while (< _value ChoixValue)
    (`/Engine/EditorBlueprintResources/StandardMacros.IncrementInt` _value
      (:`  `
        (`self.PostureAddValue` 3))))
  (set `local.Value` 0)
  (`ActorComponent.Activate` (`self.FindComponentByTag` (`self.Card`) "/Game/Blueprint/BPC/ComponentEndEffect.ComponentEndEffect_C" "End") false))

(fn `Emplacement DeckPas/Figure/Défausse`
  (params (Selection :type Integer))
  (switch `int` Selection
    (:`1`
      (set `self.Défausse Transform` (`KismetMathLibrary.MakeTransform` (520.0 430.0 0.0) (struct :`Yaw` 90.0)))
      (set `self.DeckPasTransform` (`KismetMathLibrary.MakeTransform` (230.0 430.0 0.0) (struct :`Yaw` 90.0)))
      (set `self.DeckFigure Transform` (`KismetMathLibrary.MakeTransform` (-190.0 430.0 0.0) (struct :`Yaw` 90.0)))
      (set `self.MyZoneChoréTransform` (`KismetMathLibrary.MakeTransform` (0.0 180.0 0.0) (struct :`Yaw` 90.0))))
    (:`2`
      (set `self.Défausse Transform` (`KismetMathLibrary.MakeTransform` (430.0 -550.0 0.0)))
      (set `self.DeckPasTransform` (`KismetMathLibrary.MakeTransform` (430.0 -250.0 0.0)))
      (set `self.DeckFigure Transform` (`KismetMathLibrary.MakeTransform` (430.0 150.0 0.0)))
      (set `self.MyZoneChoréTransform` (`KismetMathLibrary.MakeTransform` (180.0 0.0 0.0))))
    (:`3`
      (set `self.Défausse Transform` (`KismetMathLibrary.MakeTransform` (-530.0 -430.0 0.0) (struct :`Yaw` -90.0)))
      (set `self.DeckPasTransform` (`KismetMathLibrary.MakeTransform` (-250.0 -430.0 0.0) (struct :`Yaw` -90.0)))
      (set `self.DeckFigure Transform` (`KismetMathLibrary.MakeTransform` (170.0 -430.0 0.0) (struct :`Yaw` -90.0)))
      (set `self.MyZoneChoréTransform` (`KismetMathLibrary.MakeTransform` (0.0 -180.0 0.0) (struct :`Yaw` -90.0))))
    (:`4`
      (set `self.Défausse Transform` (`KismetMathLibrary.MakeTransform` (-430.0 510.0 0.0) (struct :`Yaw` 180.0)))
      (set `self.DeckPasTransform` (`KismetMathLibrary.MakeTransform` (-429.0 220.0 0.0) (struct :`Yaw` 180.0)))
      (set `self.DeckFigure Transform` (`KismetMathLibrary.MakeTransform` (-430.0 -160.0 0.0) (struct :`Yaw` 180.0)))
      (set `self.MyZoneChoréTransform` (`KismetMathLibrary.MakeTransform` (0.0 180.0 0.0) (struct :`Yaw` 180.0))))))

(fn `EtenduEffect`
  (params (ChoixValue :type Integer))
  (locals (carteC :type "/Game/Blueprint/ListeEtEnum/FCardInstanceDataClassique Structure") (carteB :type "/Game/Blueprint/ListeEtEnum/FCardInstanceDataBollywood Structure") (CarteVersoC :type "Array of /Game/Blueprint/ListeEtEnum/FCardInstanceDataClassique Structure") (CarteVersoB :type "Array of /Game/Blueprint/ListeEtEnum/FCardInstanceDataBollywood Structure") (carteD :type "/Game/Blueprint/ListeEtEnum/FCardInstanceDataDisco Structure") (CarteVersoD :type "Array of /Game/Blueprint/ListeEtEnum/FCardInstanceDataDisco Structure") (CarteVersoU :type "Array of /Game/Blueprint/ListeEtEnum/FCardInstanceDataUrban Structure") (carteU :type "/Game/Blueprint/ListeEtEnum/FCardInstanceDataUrban Structure"))
  (bind _playerbollywood (`/Game/Blueprint/GM_StepUP.PlayerBollywood` (`self.GM`)))
  (bind _playerdisco (`/Game/Blueprint/GM_StepUP.PlayerDisco` (`self.GM`)))
  (bind _playerurban (`/Game/Blueprint/GM_StepUP.PlayerUrban` (`self.GM`)))
  (switch `int` ChoixValue
    (:`Default`
      _)
    (:`1`
      (for _array_element (`self.PileZoneChoré`)
        (bind _output_get (set `local.carteC` _array_element))
        (if (not (`.IsRecto?_27_316E29D84EAD6D546888CBA8B72BD56A` (break `/Game/Blueprint/ListeEtEnum/FCardInstanceDataClassique` _output_get)))
          (`KismetArrayLibrary.Array_Add` (`local.CarteVersoC`) (`local.carteC`))))
      (bind _carteselec (`self.FromRandomBoardVersoToDéfausse` (`local.CarteVersoC`) (`self.PileDéfausse`) _array_element))
      (`self.RemoveCardFromBoard` _carteselec)
      (`self.PostureAddValue` -2
        (:`  `
          _)))
    (:`2`
      (for _array_element_2 (`/Game/Blueprint/DeckAndPlayer/BP_PlayerBollywood.PileZoneChoré` _playerbollywood)
        (bind _output_get_2 (set `local.carteB` _array_element_2))
        (if (not (`.IsRecto?_26_A74D402F4C6B37C9D05AAFA30D746732` (break `/Game/Blueprint/ListeEtEnum/FCardInstanceDataBollywood` _output_get_2)))
          (`KismetArrayLibrary.Array_Add` (`local.CarteVersoB`) (`local.carteB`))))
      (`/Game/Blueprint/DeckAndPlayer/BP_PlayerBollywood.FromRandomBoardVersoToDéfausse` _playerbollywood (`local.CarteVersoB`) (`/Game/Blueprint/DeckAndPlayer/BP_PlayerBollywood.PileDéfausse` (`/Game/Blueprint/GM_StepUP.PlayerBollywood` (`self.GM`))) (`local.carteB`))
      (`self.PostureAddValue` -2
        (:`  `
          _)))
    (:`3`
      (for _array_element_3 (`/Game/Blueprint/DeckAndPlayer/BP_PlayerDisco.PileZoneChoré` _playerdisco)
        (bind _output_get_3 (set `local.carteD` _array_element_3))
        (if (not (`.IsRecto?_27_EB842D9C46ED65CF51CCF79613F37952` (break `/Game/Blueprint/ListeEtEnum/FCardInstanceDataDisco` _output_get_3)))
          (`KismetArrayLibrary.Array_Add` (`local.CarteVersoD`) (`local.carteD`))))
      (`/Game/Blueprint/DeckAndPlayer/BP_PlayerDisco.FromRandomBoardVersoToDéfausse` _playerdisco (`local.CarteVersoD`) (`/Game/Blueprint/DeckAndPlayer/BP_PlayerDisco.PileDéfausse` (`/Game/Blueprint/GM_StepUP.PlayerDisco` (`self.GM`))) (`local.carteD`))
      (`self.PostureAddValue` -2
        (:`  `
          _)))
    (:`4`
      (for _array_element_4 (`/Game/Blueprint/DeckAndPlayer/BP_PlayerUrban.PileZoneChoré` _playerurban)
        (bind _output_get_4 (set `local.carteU` _array_element_4))
        (if (not (`.IsRecto?_28_63F5495E469FDE489E753FAFE753AA19` (break `/Game/Blueprint/ListeEtEnum/FCardInstanceDataUrban` _output_get_4)))
          (`KismetArrayLibrary.Array_Add` (`local.CarteVersoU`) (`local.carteU`))))
      (`/Game/Blueprint/DeckAndPlayer/BP_PlayerUrban.FromRandomBoardVersoToDéfausse` _playerurban (`local.CarteVersoU`) (`/Game/Blueprint/DeckAndPlayer/BP_PlayerUrban.PileDéfausse` (`/Game/Blueprint/GM_StepUP.PlayerUrban` (`self.GM`))) (`local.carteU`))
      (`self.PostureAddValue` -2
        (:`  `
          _))))
  (`ActorComponent.Activate` (`self.FindComponentByTag` (`self.Card`) "/Game/Blueprint/BPC/ComponentEndEffect.ComponentEndEffect_C" "End") false))

(fn `FigureCardPlayFromDeck`
  (params (find :type Integer))
  (locals (`Card Instance Classique` :type "/Game/Blueprint/ListeEtEnum/FCardInstanceDataClassique Structure"))
  (bind _card_instance_classique_cartetemplate (break `/Game/Blueprint/ListeEtEnum/FCardInstanceDataClassique` (`local.Card Instance Classique`)))
  (bind _card_instance_classique (`local.Card Instance Classique`))
  (bind (_cardboxtransfom_location _cardboxtransfom_rotation _cardboxtransfom_scale) (`KismetMathLibrary.BreakTransform` (`/Game/Blueprint/BP_PisteEtChoré.CardBoxTransfom` (`/Game/Blueprint/GM_StepUP.BP_Piste` (`self.GM`)))))
  (bind _output_get (set `local.Card Instance Classique` (`|GetArrayItem` (`self.DeckFigure`) find)))
  (`/Game/Blueprint/BP_PisteEtChoré.SelectBox` (`/Game/Blueprint/GM_StepUP.BP_Piste` (`self.GM`)))
  (bind _output_get_2 (set `local.Card Instance Classique` (make `/Game/Blueprint/ListeEtEnum/FCardInstanceDataClassique` (break `/Game/Blueprint/ListeEtEnum/FCardInstanceDataClassique` _output_get) (`.UniqueIDGUID_25_BB4736E24C37F0B39876D5B3D1914939` (break `/Game/Blueprint/ListeEtEnum/FCardInstanceDataClassique` _output_get)) (`.OwnerID_10_6FF36D9A48E4EF047131B28C579EED57` (break `/Game/Blueprint/ListeEtEnum/FCardInstanceDataClassique` _output_get)) (`.HasBeenPlayed_13_CD654ED84B51DDE833AC3794D022A5B1` (break `/Game/Blueprint/ListeEtEnum/FCardInstanceDataClassique` _output_get)) (`.DeckNumber_17_0DE01F88464E1E8634D709B000A51AF6` (break `/Game/Blueprint/ListeEtEnum/FCardInstanceDataClassique` _output_get)) (`.DeckStyle_28_A0989BCD4049946FF8EBFDB74FABDABE` (break `/Game/Blueprint/ListeEtEnum/FCardInstanceDataClassique` _output_get)) "NewEnumerator2")))
  (bind _returnvalue (`|SpawnActorFromClass` "/Game/Blueprint/BP_Cartes.BP_Cartes_C" (`KismetMathLibrary.MakeTransform` _cardboxtransfom_location _cardboxtransfom_rotation (* _cardboxtransfom_scale (7.0 8.0 6.0))) "Undefined" "MultiplyWithRoot" null (struct) (struct) _output_get_2 (struct) "NewEnumerator3" (`/Game/Blueprint/ListeEtEnum/DA_Cartes.ComponentCardEffect` _card_instance_classique_cartetemplate) (`self.GM`) false null))
  (`/Game/Blueprint/BP_PisteEtChoré.AddToPiste` :`self` (`/Game/Blueprint/GM_StepUP.BP_Piste` (`self.GM`)) :`PisteClassique` _card_instance_classique :`Style` (`.DeckStyle_28_A0989BCD4049946FF8EBFDB74FABDABE` (break `/Game/Blueprint/ListeEtEnum/FCardInstanceDataClassique` _output_get)) :`Carte` _returnvalue)
  (`self.MyZoneChoréCardInst` (`/Game/Blueprint/GM_StepUP.PlayerClassique` (`self.GM`)) _card_instance_classique)
  (`KismetArrayLibrary.Array_RemoveItem` (`self.DeckFigure`) _card_instance_classique))

(fn `FromRandomBoardVersoToDéfausse`
  (params (carteVersoC :type "Array of /Game/Blueprint/ListeEtEnum/FCardInstanceDataClassique Structure") (`PileDéfausse` :type "Array of /Game/Blueprint/ListeEtEnum/FCardInstanceDataClassique Structure (by ref)") (CarteC :type "/Game/Blueprint/ListeEtEnum/FCardInstanceDataClassique Structure"))
  (returns (CarteSelec :type "/Game/Blueprint/ListeEtEnum/FCardInstanceDataClassique Structure"))
  (locals (`Card Instance Classique` :type "/Game/Blueprint/ListeEtEnum/FCardInstanceDataClassique Structure"))
  (bind _returnvalue (`KismetArrayLibrary.Array_Length` carteVersoC))
  (bind (_card_instance_classique_cartetemplate _card_instance_classique_uniqueidguid _card_instance_classique_ownerid _card_instance_classique_hasbeenplayed _card_instance_classique_decknumber _card_instance_classique_deckstyle _card_instance_classique_location _card_instance_classique_isrecto_) (break `/Game/Blueprint/ListeEtEnum/FCardInstanceDataClassique` (`local.Card Instance Classique`)))
  (bind _output (`|GetArrayItem` carteVersoC (`KismetMathLibrary.RandomInteger` (- _returnvalue 1))))
  (set `local.Card Instance Classique` CarteC)
  (if (> _returnvalue 0)
    (`/Game/Blueprint/BP_PisteEtChoré.GestionRemoveToPLayerPiste` :`self` (`/Game/Blueprint/GM_StepUP.BP_Piste` (`self.GM`)) :`Classique` _output :`Style` "Classique")
    (`KismetArrayLibrary.Array_Add` `PileDéfausse` _output)
    (bind _output_get (set `local.Card Instance Classique` (make `/Game/Blueprint/ListeEtEnum/FCardInstanceDataClassique` _card_instance_classique_cartetemplate _card_instance_classique_uniqueidguid _card_instance_classique_ownerid _card_instance_classique_hasbeenplayed _card_instance_classique_decknumber _card_instance_classique_deckstyle "NewEnumerator3" _card_instance_classique_isrecto_)))
    (`|SpawnActorFromClass` "/Game/Blueprint/BP_Cartes.BP_Cartes_C" (`self.Défausse Transform`) "Undefined" "MultiplyWithRoot" null (struct) (struct) _output_get (struct) "NewEnumerator3" null (`self.GM`) false null)
    (return _output_get)))

(fn `GenrateZoneFigureCard`
  (locals (TailleZone :type Integer :default 2))
  (bind _deckfigure (`self.DeckFigure`))
  (bind _output (`|GetArrayItem` _deckfigure))
  (while (< (`KismetArrayLibrary.Array_Length` (`self.ZoneFigureCard`)) (`local.TailleZone`))
    (`KismetArrayLibrary.Array_Add` (`self.ZoneFigureCard`) _output)
    (`KismetArrayLibrary.Array_RemoveItem` _deckfigure _output)))

(fn `Gestion Carte Data Défausse`
  (params (cardInstance :type "/Game/Blueprint/ListeEtEnum/FCardInstanceDataClassique Structure"))
  (`KismetArrayLibrary.Array_Add` (`self.PileDéfausse`) cardInstance))

(fn `GestionLimiteCarteJouéParTour`
  (bind _result (`/Engine/EditorBlueprintResources/StandardMacros.IncrementInt` (`self.CarteJoué`))
    (:`  `
      (if (>= _result 3)
        (set `/Game/Blueprint/Widget/WBPStyle/WBP_ClassiqueHand.MaxCard` true (`/Game/Blueprint/GM_StepUP.WBP Classique` (`self.GM`)))))))

(fn `GestionnaireDeChoix`
  (params (ValueChoix :type Integer))
  (locals (ActualCardEffect :type "/Game/Blueprint/ListeEtEnum/FCardInstanceDataClassique Structure") (Value :type Integer))
  (bind _value (`local.Value`))
  (bind `_cartezonechoréclassique` (`/Game/Blueprint/BP_PisteEtChoré.CarteZoneChoréClassique` (`/Game/Blueprint/GM_StepUP.BP_Piste` (`self.GM`))))
  (set `self.ValueCheck` ValueChoix)
  (set `local.Value` ValueChoix)
  (if (`self.OnPassifEffect`)
    (`self.défaussePassifClasique` (`local.Value`))
    (else
      (bind _output_get (set `local.ActualCardEffect` (`|GetArrayItem` `_cartezonechoréclassique` (- (`KismetArrayLibrary.Array_Length` `_cartezonechoréclassique`) 1))))
      (switch `string` (`KismetTextLibrary.Conv_TextToString` (`/Game/Blueprint/ListeEtEnum/DA_Cartes.CardName` (break `/Game/Blueprint/ListeEtEnum/FCardInstanceDataClassique` _output_get)))
        (:`Plié`
          (`self.PliéEffect` _value))
        (:`Elegant`
          (`/Game/Blueprint/Widget/WBPStyle/WBP_ClassiqueHand.handCardSelect` (`/Game/Blueprint/GM_StepUP.WBP Classique` (`self.GM`)) _value))
        (:`Etendu`
          (`self.EtenduEffect` _value))))))

(fn `MyZoneChoréCardInst`
  (params (`cardInstChoré` :type "/Game/Blueprint/ListeEtEnum/FCardInstanceDataClassique Structure"))
  (`KismetArrayLibrary.Array_Add` (`self.PileZoneChoré`) `cardInstChoré`))

(fn `PassifClassique`
  (locals (Range4 :type Integer) (postureUp :type Integer)))

(fn `PliéEffect`
  (params (ChoixValue :type Integer))
  (locals (Value :type Integer))
  (while (< (`local.Value`) ChoixValue)
    (`/Engine/EditorBlueprintResources/StandardMacros.IncrementInt` (`local.Value`)
      (:`  `
        (`self.PostureAddValue` -1
          (:`  `
            (set `self.AdeptesClassique` (+ (`self.AdeptesClassique`) 3)))))))
  (set `local.Value` 0)
  (`ActorComponent.Activate` (`self.FindComponentByTag` (`self.Card`) "/Game/Blueprint/BPC/ComponentEndEffect.ComponentEndEffect_C" "End") false))

(fn `PostureAddValueF`
  (params (PostureValue :type Integer))
  (bind _jeton (`self.Jeton`))
  (bind _output_get (set `self.Posture` (+ (`BlueprintMapLibrary.Map_Find` (`self.Jeton`) "Posture") PostureValue)))
  (`BlueprintMapLibrary.Map_Remove` _jeton "Posture")
  (`BlueprintMapLibrary.Map_Add` _jeton "Posture" _output_get))

(fn `ReadAndActiveCardEffect`
  (params (Card :type "/Game/Blueprint/BP_Cartes Object Reference"))
  (bind _output_get (set `self.Card` Card))
  (`ActorComponent.Activate` (`self.FindComponentByTag` _output_get "/Game/Blueprint/BPC/ComponentCardEffect.ComponentCardEffect_C" "CardEffect") false))

(fn `RefMain`
  (params (Main :type "Array of /Game/Blueprint/ListeEtEnum/FCardInstanceDataClassique Structure"))
  (set `self.HandCarte` Main))

(fn `RemoveCardFromBoard`
  (params (`Classique Card` :type "/Game/Blueprint/ListeEtEnum/FCardInstanceDataClassique Structure"))
  (locals (cardClassique :type "/Game/Blueprint/ListeEtEnum/FCardInstanceDataClassique Structure"))
  (bind (_cardclassique_cartetemplate _cardclassique_uniqueidguid _cardclassique_ownerid _cardclassique_hasbeenplayed _cardclassique_decknumber _cardclassique_deckstyle) (break `/Game/Blueprint/ListeEtEnum/FCardInstanceDataClassique` (`local.cardClassique`)))
  (bind _output_get (set `local.cardClassique` `Classique Card`))
  (`/Game/Blueprint/BP_PisteEtChoré.GestionRemoveToPLayerPiste` :`self` (`/Game/Blueprint/GM_StepUP.BP_Piste` (`self.GM`)) :`Classique` _output_get :`Style` _cardclassique_deckstyle)
  (set `/Game/Blueprint/BP_PisteEtChoré.CarteZoneChoréClassique` (`self.PileZoneChoré`) (`/Game/Blueprint/GM_StepUP.BP_Piste` (`self.GM`))))

(fn `RemoveCardhandToDéfausse`
  (params (carte :type "/Game/Blueprint/Widget/WBP_Cartes Object Reference"))
  (bind (_cardinstanceclassique_cartetemplate _cardinstanceclassique_uniqueidguid _cardinstanceclassique_ownerid _cardinstanceclassique_hasbeenplayed _cardinstanceclassique_decknumber _cardinstanceclassique_deckstyle _cardinstanceclassique_location _cardinstanceclassique_isrecto_) (break `/Game/Blueprint/ListeEtEnum/FCardInstanceDataClassique` (`/Game/Blueprint/Widget/WBP_Cartes.CardInstanceClassique` carte)))
  (`KismetArrayLibrary.Array_RemoveItem` (`self.HandCarte`) (`/Game/Blueprint/Widget/WBP_Cartes.CardInstanceClassique` carte))
  (`KismetArrayLibrary.Array_Add` (`self.PileDéfausse`) (make `/Game/Blueprint/ListeEtEnum/FCardInstanceDataClassique` _cardinstanceclassique_cartetemplate _cardinstanceclassique_uniqueidguid _cardinstanceclassique_ownerid _cardinstanceclassique_hasbeenplayed _cardinstanceclassique_decknumber _cardinstanceclassique_deckstyle "NewEnumerator3" _cardinstanceclassique_isrecto_))
  (`Widget.RemoveFromParent` carte))

(fn `ShufflePas`
  (`KismetArrayLibrary.Array_Shuffle` (`self.DeckPas`)))

(fn `SplitDeckPas/Figure`
  (params (CardInstance :type "Array of /Game/Blueprint/ListeEtEnum/FCardInstanceDataClassique Structure"))
  (bind (_sdatacard_cartetemplate _sdatacard_uniqueidguid _sdatacard_ownerid _sdatacard_hasbeenplayed _sdatacard_decknumber _sdatacard_deckstyle _sdatacard_location _sdatacard_isrecto_) (break `/Game/Blueprint/ListeEtEnum/FCardInstanceDataClassique` (`self.SDataCard`)))
  (for _array_element CardInstance
    (bind _output_get (set `self.SDataCard` _array_element))
    (if (`|EnumEquality` (`self.EType`) (`/Game/Blueprint/ListeEtEnum/DA_Cartes.CardType` (break `/Game/Blueprint/ListeEtEnum/FCardInstanceDataClassique` _output_get)))
      (bind _output_get_2 (set `self.SDataCard` (make `/Game/Blueprint/ListeEtEnum/FCardInstanceDataClassique` _sdatacard_cartetemplate _sdatacard_uniqueidguid _sdatacard_ownerid _sdatacard_hasbeenplayed _sdatacard_decknumber _sdatacard_deckstyle "NewEnumerator5" _sdatacard_isrecto_)))
      (`KismetArrayLibrary.Array_Add` (`self.DeckPas`) _output_get_2)
      (else
        (bind _output_get_3 (set `self.SDataCard` (make `/Game/Blueprint/ListeEtEnum/FCardInstanceDataClassique` _sdatacard_cartetemplate _sdatacard_uniqueidguid _sdatacard_ownerid _sdatacard_hasbeenplayed _sdatacard_decknumber _sdatacard_deckstyle "NewEnumerator0" _sdatacard_isrecto_)))
        (`KismetArrayLibrary.Array_Add` (`self.DeckFigure`) _output_get_3)))))

(fn `StartdéfaussePassifClasique`
  (set `self.OnPassifEffect` true)
  (bind _returnvalue (`|CreateWidget` "/Game/Blueprint/Widget/WBP_ChoixEffect.WBP_ChoixEffect_C" null self null null null true))
  (`UserWidget.AddToViewport` _returnvalue 0))

(fn `TransPostureToADepte`
  (set `self.AdeptesClassique` (+ (`self.AdeptesClassique`) (`BlueprintMapLibrary.Map_Find` (`self.Jeton`) "Posture")))
  (bind _values (`BlueprintMapLibrary.Map_Values` (`self.Jeton`)))
  (`KismetSystemLibrary.PrintString` (`KismetStringLibrary.Conv_IntToString` (`|GetArrayItem` _values 2)))
  (`KismetArrayLibrary.Array_Set` _values 2))

(fn `UserConstructionScript`)