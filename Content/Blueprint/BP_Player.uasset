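; BP_Player is a player Blueprint represented by a colored cube, which can be human or bot controlled.
; On BeginPlay it copies the Bot flag from its GM reference, then calls CouleurPlayer.
; CouleurPlayer switches on PlayerID, covering four players, and assigns each a distinct material on the Cube to tell them apart.
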(event `self.ReceiveBeginPlay`
  ;[0.15 0.07258 0 0.5] défini si il s'agit d'un bot ou non, puis lui attribue une couleur différente selon so n ID
  (if (`/Game/Blueprint/GM_StepUP.Bot?` (`self.GM`))
    (set `self.Bot?` true)
    (else
      (set `self.Bot?` false)))
  (`self.CouleurPlayer`))

(fn `CouleurPlayer`
  (bind _cube (`self.Cube`))
  ;[0.15 0.009671 0 0.5] Définie une couleur au cube
  (switch `int` (`self.PlayerID`)
    (:`1`
      (`PrimitiveComponent.SetMaterial` _cube 0 "/Game/MaterialEtTexture/Material/MatUniversal/Mat_UniOpaque/M_UniveralOpaque1.M_UniveralOpaque1"))
    (:`2`
      (`PrimitiveComponent.SetMaterial` _cube 0 "/Game/MaterialEtTexture/Material/MatUniversal/Mat_UniOpaque/M_UniveralOpaque1_Inst.M_UniveralOpaque1_Inst"))
    (:`3`
      (`PrimitiveComponent.SetMaterial` _cube 0 "/Game/MaterialEtTexture/Material/MatUniversal/Mat_UniOpaque/M_UniveralOpaque1_Inst1.M_UniveralOpaque1_Inst1"))
    (:`4`
      (`PrimitiveComponent.SetMaterial` _cube 0 "/Game/MaterialEtTexture/Material/MatUniversal/Mat_UniOpaque/M_UniveralOpaque1_Inst2.M_UniveralOpaque1_Inst2"))))

(fn `UserConstructionScript`)