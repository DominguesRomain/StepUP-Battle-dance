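; BP_CamMana is a camera manager that eases its Camera component between preset views.
; MoveCamToZoneTarget blends to a supplied transform, while CameraTurn simply forwards to the game mode reference's CameraTurnPlayer.
; CamZoneChoréIN and Out switch between a fixed overhead view and the player spawn transform held by GM.
; Each switch stops the opposing MoveComponentTo before starting its own, so transitions can interrupt each other.
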(event `CameraTurn`
  (`/Game/Blueprint/GM_StepUP.CameraTurnPlayer` (`self.GM`)))

(event `MoveCamToZoneTarget`
  (params (`DéfauePose` :type "Transform Structure"))
  (`KismetSystemLibrary.MoveComponentTo` (`self.Camera`) `DéfauePose_Location` `DéfauePose_Rotation` true true 0.5 true))

(event `self.ReceiveBeginPlay`)

(event `CamZoneChoréIN`
  (bind _camera (`self.Camera`))
  (bind (_spawnplayertrans_location _spawnplayertrans_rotation) (`KismetMathLibrary.BreakTransform` (`/Game/Blueprint/GM_StepUP.SpawnPlayerTrans` (`self.GM`))))
  (`|ExecutionSequence`
    (:`then_0`
      (goto _label_2 :!via `Stop`))
    (:`then_1`
      (`KismetSystemLibrary.MoveComponentTo` _camera (0.0 0.0 500.0) (struct :`Pitch` -90.0 :`Yaw` -90.0) true true 0.5 true :!label _label))))

(event `CamZoneChoréOut`
  (bind (_spawnplayertrans_location _spawnplayertrans_rotation) (`KismetMathLibrary.BreakTransform` (`/Game/Blueprint/GM_StepUP.SpawnPlayerTrans` (`self.GM`))))
  (`|ExecutionSequence`
    (:`then_0`
      (goto _label :!via `Stop`))
    (:`then_1`
      (`KismetSystemLibrary.MoveComponentTo` (`self.Camera`) _spawnplayertrans_location _spawnplayertrans_rotation true true 0.5 true :!label _label_2))))

(fn `UserConstructionScript`)