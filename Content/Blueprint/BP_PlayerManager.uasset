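; BP_PlayerManager spawns the player actor for one of four styles: Classique, Urban, Disco or Bollywood.
; On BeginPlay it copies the Bot flag from GM.
; The linkPlayerAndStyle event stores the given style and spawns the matching player class at the manager's transform, passing in GM and the style.
; It saves the new actor in that style's reference on both GM and itself.
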(event `self.ReceiveBeginPlay`
  ;[0.15 0.07258 0 0.5] défini si il s'agit d'un bot ou non, puis lui attribue une couleur différente selon so n ID
  (if (`/Game/Blueprint/GM_StepUP.Bot?` (`self.GM`))
    (set `self.Bot?` true)
    (else
      (set `self.Bot?` false))))

(event `linkPlayerAndStyle`
  (params (Style :type String))
  (bind _returnvalue (`self.GetTransform`))
  (bind _gm (`self.GM`))
  (bind _gm_2 (`self.GM`))
  ;[0.15 0.07258 0 0.5] défini si il s'agit d'un bot ou non, puis lui attribue une couleur différente selon so n ID
  (bind _output_get (set `self.style` Style))
  (switch `string` _output_get
    (:`Classique`
      (bind _returnvalue_2 (`|SpawnActorFromClass` "/Game/Blueprint/DeckAndPlayer/BP_PlayerClassique.BP_PlayerClassique_C" _returnvalue "AlwaysSpawn" "MultiplyWithRoot" null _gm _output_get null))
      (bind _output_get_2 (set `/Game/Blueprint/GM_StepUP.PlayerClassique` _returnvalue_2 _gm))
      (set `self.PlayerClassique` _output_get_2))
    (:`Urban`
      (bind _returnvalue_3 (`|SpawnActorFromClass` "/Game/Blueprint/DeckAndPlayer/BP_PlayerUrban.BP_PlayerUrban_C" _returnvalue "AlwaysSpawn" "MultiplyWithRoot" null _gm _output_get null))
      (bind _output_get_3 (set `/Game/Blueprint/GM_StepUP.PlayerUrban` _returnvalue_3 _gm))
      (set `self.PlayerUrban` _output_get_3))
    (:`Disco`
      (bind _returnvalue_4 (`|SpawnActorFromClass` "/Game/Blueprint/DeckAndPlayer/BP_PlayerDisco.BP_PlayerDisco_C" _returnvalue "AdjustIfPossibleButAlwaysSpawn" "MultiplyWithRoot" null _gm_2 _output_get null))
      (bind _output_get_4 (set `/Game/Blueprint/GM_StepUP.PlayerDisco` _returnvalue_4 _gm_2))
      (set `self.PlayerDisco` _output_get_4))
    (:`Bollywood`
      (bind _returnvalue_5 (`|SpawnActorFromClass` "/Game/Blueprint/DeckAndPlayer/BP_PlayerBollywood.BP_PlayerBollywood_C" _returnvalue "AlwaysSpawn" "MultiplyWithRoot" null _gm_2 _output_get null))
      (bind _output_get_5 (set `/Game/Blueprint/GM_StepUP.PlayerBollywood` _returnvalue_5 _gm_2))
      (set `self.PlayerBollywood` _output_get_5))))

(fn `UserConstructionScript`)