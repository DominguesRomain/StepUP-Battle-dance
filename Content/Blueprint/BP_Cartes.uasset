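; Card actor for a card game with four dance styles, shown as a flattened cube that animates into its slot.
; CardNewPlace stores the instance and moves the cube; cards from play also get an effect component linked to the game manager.
; Dynamic materials show artwork or a back texture according to IsRecto, and ChangeFace applies the opposite face.
; CardDestroy removes the card from BPPiste and notifies that style's widget.
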(event `CardNewPlace`
  (params (trans :type "Transform Structure") (Instance :type "/Game/Blueprint/ListeEtEnum/FCardInstanceData Structure"))
  (bind (_cartesinstance_cartetemplate _cartesinstance_ownerid _cartesinstance_decknumber _cartesinstance_deckstyle _cartesinstance_location _cartesinstance_isrecto_) (break `/Game/Blueprint/ListeEtEnum/FCardInstanceData` (`self.CartesInstance`)))
  (bind _cube (`self.Cube`))
  (set `self.CartesInstance` Instance)
  (`SceneComponent.SetWorldScale3D` _cube (0.45 0.33 0.02))
  (`KismetSystemLibrary.MoveComponentTo` _cube trans_Location (`KismetMathLibrary.MakeRotator` (.roll (.rotation trans)) (.pitch (.rotation trans)) (+ (.yaw (.rotation trans)) 90.0)) false false 0.4)
  (if (`self.FromPlay`) :!label _label
    (bind _returnvalue (`|AddComponentByClass` (`self.Component`) self (`self.GM`)))
    (set `self.ComponentActiveEffect` _returnvalue))
  (if _cartesinstance_isrecto_
    (bind _returnvalue_2 (`PrimitiveComponent.CreateDynamicMaterialInstance` (`self.Cube`) 0 "/Game/MaterialEtTexture/Material/MatUniversal/Mat_UniMasque/M_CardMaskUni_Inst.M_CardMaskUni_Inst" "Moi" :!label _label_2))
    (`MaterialInstanceDynamic.SetTextureParameterValue` _returnvalue_2 "TextureCard" (`/Game/Blueprint/ListeEtEnum/DA_Cartes.Artwork` _cartesinstance_cartetemplate))
    (`MaterialInstanceDynamic.SetScalarParameterValue` _returnvalue_2 "StartTime" (`KismetSystemLibrary.GetGameTimeInSeconds`))
    (`/Engine/EditorBlueprintResources/StandardMacros.DoOnce` false)
    (else
      (bind _returnvalue_3 (`PrimitiveComponent.CreateDynamicMaterialInstance` (`self.Cube`) 0 "/Game/MaterialEtTexture/Material/MatUniversal/Mat_UniMasque/M_CardMaskUni_Inst.M_CardMaskUni_Inst" "Moi" :!label _label_3))
      (`MaterialInstanceDynamic.SetTextureParameterValue` _returnvalue_3 "TextureCard" "/Game/MaterialEtTexture/Texture/Cartes/250.250")
      (`MaterialInstanceDynamic.SetScalarParameterValue` _returnvalue_3 "StartTime" (`KismetSystemLibrary.GetGameTimeInSeconds`))
      (`/Engine/EditorBlueprintResources/StandardMacros.DoOnce` false))))

(event `ChangeFace`
  (bind (_cartesinstance_cartetemplate _cartesinstance_ownerid _cartesinstance_decknumber _cartesinstance_deckstyle _cartesinstance_location _cartesinstance_isrecto_) (break `/Game/Blueprint/ListeEtEnum/FCardInstanceData` (`self.CartesInstance`)))
  (if (not _cartesinstance_isrecto_)
    (goto _label_2)
    (else
      (goto _label_3))))

(event `self.ReceiveBeginPlay`
  (goto _label))

(event `/Game/Blueprint/BPI/BPI_WidgetInter.CardDestroy`
  (params (Card :type "/Game/Blueprint/BP_Cartes Object Reference"))
  (bind _gm (`self.GM`))
  (bind _cartesinstance (`self.CartesInstance`))
  (bind _style (`self.Style`))
  (bind _bp_piste (`/Game/Blueprint/GM_StepUP.BP_Piste` _gm))
  (switch `/Game/Blueprint/ListeEtEnum/E_Style` _style
    (:`NewEnumerator0`
      (`/Game/Blueprint/BP_PisteEtChoré.GestionRemoveToPLayerPiste` _bp_piste _style _cartesinstance)
      (message `/Game/Blueprint/BPI/BPI_WidgetInter.CardDestroy` (`/Game/Blueprint/GM_StepUP.WBP Disco` _gm) Card))
    (:`NewEnumerator1`
      (`/Game/Blueprint/BP_PisteEtChoré.GestionRemoveToPLayerPiste` _bp_piste _style _cartesinstance)
      (message `/Game/Blueprint/BPI/BPI_WidgetInter.CardDestroy` (`/Game/Blueprint/GM_StepUP.WBP Bollywood` _gm) Card))
    (:`NewEnumerator2`
      (`/Game/Blueprint/BP_PisteEtChoré.GestionRemoveToPLayerPiste` _bp_piste _style _cartesinstance)
      (message `/Game/Blueprint/BPI/BPI_WidgetInter.CardDestroy` (`/Game/Blueprint/GM_StepUP.WBP Urban` _gm) Card))
    (:`NewEnumerator3`
      (`/Game/Blueprint/BP_PisteEtChoré.GestionRemoveToPLayerPiste` _bp_piste _style _cartesinstance)
      (message `/Game/Blueprint/BPI/BPI_WidgetInter.CardDestroy` (`/Game/Blueprint/GM_StepUP.WBP Classique` _gm) Card))))

(event `self.ComponentEndEffect.OnComponentActivated`
  (params (Component :type "ActorComponent Object Reference") (bReset :type Boolean))
  (set `/Game/Blueprint/BPC/ComponentEndEffect.card` self (`self.ComponentEndEffect`)))

(fn `UserConstructionScript`)